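; FatherBp is an actor Blueprint, apparently meant as a parent class, that shows a text label when the first-person character is near.
; Capsule overlap begin and end events set the IsOverlap flag for FirstPersonCharacter only.
; Each Tick, a valid TextRender takes its visibility from that flag and turns to face the player, using look-at yaw plus a half turn with pitch held flat.
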(event `self.ReceiveTick`
  (params (DeltaSeconds :type "Float (single-precision)"))
  (bind _textrender (`self.TextRender`))
  (if (`KismetSystemLibrary.IsValid` _textrender)
    (`SceneComponent.K2_SetRelativeRotation` _textrender (`KismetMathLibrary.MakeRotator` (.roll (`KismetMathLibrary.FindLookAtRotation` (`self.K2_GetActorLocation` (`GameplayStatics.GetPlayerCharacter` 0)) (`self.K2_GetActorLocation`))) 0.0 (+ (.yaw (`KismetMathLibrary.FindLookAtRotation` (`self.K2_GetActorLocation` (`GameplayStatics.GetPlayerCharacter` 0)) (`self.K2_GetActorLocation`))) 180.0)) false false)
    (`SceneComponent.SetVisibility` (`self.TextRender`) (`self.isOverlap`) false)))

(event `self.Capsule.OnComponentBeginOverlap`
  (params (OverlappedComponent :type "PrimitiveComponent Object Reference") (OtherActor :type "Actor Object Reference") (OtherComp :type "PrimitiveComponent Object Reference") (OtherBodyIndex :type Integer) (bFromSweep :type Boolean) (SweepResult :type "HitResult Structure (by ref)"))
  (cast `/Game/ThirdPersonBP/Blueprints/FirstPersonCharacter` OtherActor)
  (set `self.isOverlap` true))

(event `self.Capsule.OnComponentEndOverlap`
  (params (OverlappedComponent :type "PrimitiveComponent Object Reference") (OtherActor :type "Actor Object Reference") (OtherComp :type "PrimitiveComponent Object Reference") (OtherBodyIndex :type Integer))
  (cast `/Game/ThirdPersonBP/Blueprints/FirstPersonCharacter` OtherActor)
  (set `self.isOverlap` false))

(fn `UserConstructionScript`)